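; BP_VFX_GhostDie is a short-lived effect actor that plays a ghost death animation through Niagara.
; StartDeathAnim makes its skeletal mesh mirror the target's transform and mesh, following its pose as master component.
; It attaches a Niagara system, feeding that copy and a second passed-in actor's mesh as the two skeletal mesh user variables.
; Bounds are scaled up hugely, and a timer destroys the actor shortly afterwards.
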(fn `Finish`
  (`self.K2_DestroyActor`))

(fn `StartDeathAnim`
  (params (Target :type "SkinnedMeshComponent Object Reference") (NewParam :type "/Game/GameJam/Blueprints/Character/BP_TestCharacter Object Reference"))
  (bind _skeletalmesh (`self.SkeletalMesh`))
  (`SceneComponent.K2_SetRelativeTransform` (`self.SkeletalMesh`) (`SceneComponent.GetRelativeTransform` Target) false false)
  (`SkinnedMeshComponent.SetSkinnedAssetAndUpdate` _skeletalmesh (`SkinnedMeshComponent.SkeletalMesh` Target) false)
  (`SkinnedMeshComponent.SetLeaderPoseComponent` _skeletalmesh Target false)
  (bind _returnvalue (`NiagaraFunctionLibrary.SpawnSystemAttached` "/Game/GameJam/VFXs/NewNiagaraSystem.NewNiagaraSystem" (`self.SkeletalMesh`) "None" (0.0 0.0 0.0) (struct) "SnapToTarget" true true "None" false))
  (bind _output_get (set `self.VFX` _returnvalue))
  (`NiagaraFunctionLibrary.OverrideSystemUserVariableSkeletalMeshComponent` _returnvalue "User.MESHA" (`self.SkeletalMesh`))
  (`NiagaraFunctionLibrary.OverrideSystemUserVariableSkeletalMeshComponent` _returnvalue "User.MESHB" (`Character.Mesh` NewParam))
  (`KismetSystemLibrary.K2_SetTimer` null "Finish" 2.0)
  (`PrimitiveComponent.SetBoundsScale` _output_get 2000.0))

(fn `UserConstructionScript`)