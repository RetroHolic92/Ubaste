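; BP_LandLight is a land light that acts as one of several switches for the final gate.
; It starts dim through a dynamic material's emissive intensity, and InterOpenGate brightens it and sets CanOpen.
; It then ANDs CanOpen across all actors tagged Light into OpenGate.
; If that is true, it calls CEStartRotation on BP_Gate actors tagged FinalGate.
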(event `self.ReceiveBeginPlay`
  (bind _sm_landlight (`self.SM_LandLight`))
  (bind _returnvalue (`PrimitiveComponent.CreateDynamicMaterialInstance` _sm_landlight 0 (`PrimitiveComponent.GetMaterial` _sm_landlight 0) "None"))
  (set `self.MaterialInstance` _returnvalue)
  (`MaterialInstanceDynamic.SetScalarParameterValue` (`self.MaterialInstance`) "EmissIntensity" 0.005))

(event `/Game/GameJam/Blueprints/Item/Inter_Gate.Inter_OpenGate`
  (params (ID :type Boolean))
  (`self.OpenLight`)
  (set `self.bCanOpen` true)
  (bind _outactors (`GameplayStatics.GetAllActorsWithTag` "Light"))
  (for _array_element _outactors
    (bind _asbp_land_light (cast `/Game/GameJam/Blueprints/Item/Light/BP_LandLight` _array_element))
    (set `self.bOpenGate` (and (`/Game/GameJam/Blueprints/Item/Light/BP_LandLight.bCanOpen` _asbp_land_light) (`self.bOpenGate`))))
  (if (`self.bOpenGate`)
    (bind _outactors_2 (`GameplayStatics.GetAllActorsWithTag` "FinalGate"))
    (for _array_element_2 _outactors_2
      (bind _asbp_gate (cast `/Game/GameJam/Blueprints/Item/BP_Gate` _array_element_2))
      (`/Game/GameJam/Blueprints/Item/BP_Gate.CE_StartRotation` _asbp_gate))))

(event `OpenLight`
  (`MaterialInstanceDynamic.SetScalarParameterValue` (`self.MaterialInstance`) "EmissIntensity" 50.0))

(fn `UserConstructionScript`)