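; BP_EndLevel is a level-end trigger that fires when the BP_TestCharacter overlaps its Box component.
; The overlap disables the character's input and spawns a particle system at the box, stored as FallingCat so it is not respawned while still valid.
; It then passes NextLevel to the game mode to stop the game timer and to the player controller to show the end-level UI.
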(event `self.ReceiveBeginPlay`)

(event `self.Box.OnComponentBeginOverlap`
  (params (OverlappedComponent :type "PrimitiveComponent Object Reference") (OtherActor :type "Actor Object Reference") (OtherComp :type "PrimitiveComponent Object Reference") (OtherBodyIndex :type Integer) (bFromSweep :type Boolean) (SweepResult :type "HitResult Structure (by ref)"))
  (bind _asbp_test_character (cast `/Game/GameJam/Blueprints/Character/BP_TestCharacter` OtherActor))
  (`self.DisableInput` _asbp_test_character (`GameplayStatics.GetPlayerController` 0))
  (`|ExecutionSequence`
    (:`then_0`
      (`self.FallingCat`
        (:`then`)
        (:`else`
          (bind _returnvalue (`NiagaraFunctionLibrary.SpawnSystemAtLocation` "/Game/ExampleContent/Niagara/PBD/PBD.PBD" (`SceneComponent.K2_GetComponentLocation` (`self.Box`))))
          (set `self.FallingCat` _returnvalue))))
    (:`then_1`
      (bind _asbp_third_person_game_mode (cast `/Game/ThirdPerson/Blueprints/BP_ThirdPersonGameMode` (`GameplayStatics.GetGameMode`)))
      (`/Game/ThirdPerson/Blueprints/BP_ThirdPersonGameMode.StopCountGameTime` _asbp_third_person_game_mode (`self.NextLevel`)))
    (:`then_2`
      (bind _asbp_pc_game (cast `/Game/GameJam/Blueprints/GM/BP_PC_Game` (`GameplayStatics.GetPlayerController` 0)))
      (`/Game/GameJam/Blueprints/GM/BP_PC_Game.ShowEndLevelUI` _asbp_pc_game (`self.NextLevel`)))))

(fn `ComponentsToSave`
  (returns (Components :type "Array of ActorComponent Object Reference"))
  (return))

(fn `UserConstructionScript`)