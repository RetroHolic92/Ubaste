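; Sign board actor that shows a widget while a character stands inside its trigger box.
; On BeginPlay it creates the configured SignWidget, assigns it to the Widget1 component and hides it.
; Box overlap by a Character shows the component, and any end overlap hides it again.
; Disconnected leftovers, including calls to SetRenderLocation, hold an older screen-projected viewport widget approach with timeline scaling.
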(event `self.ReceiveBeginPlay`
  (bind _returnvalue (`|CreateWidget` (`self.SignWidget_`)))
  (`WidgetComponent.SetWidget` (`self.Widget1`) _returnvalue)
  (`SceneComponent.SetVisibility` (`self.Widget1`) false false))

(event `self.Box.OnComponentBeginOverlap`
  (params (OverlappedComponent :type "PrimitiveComponent Object Reference") (OtherActor :type "Actor Object Reference") (OtherComp :type "PrimitiveComponent Object Reference") (OtherBodyIndex :type Integer) (bFromSweep :type Boolean) (SweepResult :type "HitResult Structure (by ref)"))
  (cast `Character` OtherActor)
  (`SceneComponent.SetVisibility` (`self.Widget1`) true false))

(event `self.Box.OnComponentEndOverlap`
  (params (OverlappedComponent :type "PrimitiveComponent Object Reference") (OtherActor :type "Actor Object Reference") (OtherComp :type "PrimitiveComponent Object Reference") (OtherBodyIndex :type Integer))
  (`SceneComponent.SetVisibility` (`self.Widget1`) false false))

(event `self.ReceiveTick`
  (params (DeltaSeconds :type "Float (single-precision)")))

(fn `SetRenderLocation`
  (params (Widget :type "UserWidget Object Reference"))
  (bind _returnvalue (`WidgetLayoutLibrary.GetViewportScale`))
  (`Widget.SetRenderTransform` (`/Game/GameJam/Blueprints/UI/SignWidget/WBP_SignMain.Image_Tips` (cast `/Game/GameJam/Blueprints/UI/SignWidget/WBP_SignMain` Widget :!pure true)) (make `WidgetTransform` (/ (`GameplayStatics.ProjectWorldToScreen` (`GameplayStatics.GetPlayerController` 0) (`SceneComponent.K2_GetComponentLocation` (`self.Scene`)) true) (`KismetMathLibrary.MakeVector2D` _returnvalue _returnvalue)) (`self.Scale`))))

(fn `UserConstructionScript`)