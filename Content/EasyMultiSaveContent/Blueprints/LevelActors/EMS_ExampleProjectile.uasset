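; Example physics projectile for the Easy Multi Save system, showing how a moving, colored actor keeps its state through save and load.
; ActorPreSave stores the physics sphere's linear velocity in a variable, and ActorLoaded re-applies it so the motion resumes.
; The construction script creates a dynamic material instance and applies the Color variable, which is also re-applied after loading.
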(event `EMSActorSaveInterface.ActorPreSave`
  ;[1 1 1] Save and Re-Apply Linear Velocity
  (bind _returnvalue (`PrimitiveComponent.GetPhysicsLinearVelocity` (`self.PhysicsSphere`) "None"))
  (set `self.SavedLinearVelocity` _returnvalue))

(event `EMSActorSaveInterface.ActorLoaded`
  ;[1 1 1] Save and Re-Apply Linear Velocity
  (`PrimitiveComponent.SetPhysicsLinearVelocity` (`self.PhysicsSphere`) (`self.SavedLinearVelocity`) false "None")
  (`self.Set Color`) ; The color variable is set on spawn and in the level and also saved
)

(fn `ComponentsToSave`
  (returns (Components :type "Array of ActorComponent Object Reference"))
  (return))

(fn `Set Color`
  (`MaterialInstanceDynamic.SetVectorParameterValue` (`self.MaterialInstance`) "Color" (`self.Color`)))

(fn `UserConstructionScript`
  (bind _returnvalue (`PrimitiveComponent.CreateDynamicMaterialInstance` (`self.PhysicsSphere`) 0 null "None"))
  (set `self.MaterialInstance` _returnvalue)
  (`self.Set Color`))