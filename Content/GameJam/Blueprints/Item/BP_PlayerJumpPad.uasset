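; BP_PlayerJumpPad is a jump pad that launches the player's test character upward.
; When its Box is overlapped by a BP_TestCharacter, it calls LaunchCharacter with JumpHeight as vertical velocity, overriding existing velocity on all axes, and plays a 2D jump sound.
; The IsJumped guard is never set by live code, since its setters and an alternative impulse-based launch are disconnected.
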(event `self.Box.OnComponentBeginOverlap`
  (params (OverlappedComponent :type "PrimitiveComponent Object Reference") (OtherActor :type "Actor Object Reference") (OtherComp :type "PrimitiveComponent Object Reference") (OtherBodyIndex :type Integer) (bFromSweep :type Boolean) (SweepResult :type "HitResult Structure (by ref)"))
  (if (not (`self.IsJumped`))
    (bind _asbp_test_character (cast `/Game/GameJam/Blueprints/Character/BP_TestCharacter` OtherActor))
    (`Character.LaunchCharacter` _asbp_test_character (`KismetMathLibrary.MakeVector` 0.0 0.0 (`self.JumpHeight`)) true true)
    (`GameplayStatics.PlaySound2D` "/Game/GameJam/Audio/jump.jump" 1.0 1.0 0.0 null null)))

(event `self.Box.OnComponentEndOverlap`
  (params (OverlappedComponent :type "PrimitiveComponent Object Reference") (OtherActor :type "Actor Object Reference") (OtherComp :type "PrimitiveComponent Object Reference") (OtherBodyIndex :type Integer)))

(fn `UserConstructionScript`)