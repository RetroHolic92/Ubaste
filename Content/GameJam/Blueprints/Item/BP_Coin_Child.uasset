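; BP_Coin_Child is a coin item child Blueprint that plays a reward animation when triggered.
; Its Triggered override starts a custom event, then calls the parent implementation.
; The event shows the static mesh and runs a timeline driving its scale, roll and height, plus the height of a Scene component.
; When the timeline finishes, it hides the mesh, spawns a Niagara effect at its location and plays a coin sound.
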(event `self.ReceiveBeginPlay`
  (`parent.ReceiveBeginPlay`))

(event `CustomEvent_0`
  (`SceneComponent.SetVisibility` (`self.StaticMesh`) true false)
  (bind (_direction _newtrack_0 _newtrack_1 _newtrack_2 _newtrack_3) (`Timeline|Timeline_0` :!via `PlayFromStart`)
    (:`Update`
      (`SceneComponent.SetWorldScale3D` (`self.StaticMesh`) _newtrack_0)
      (`SceneComponent.K2_SetWorldRotation` (`self.StaticMesh`) (`KismetMathLibrary.MakeRotator` _newtrack_1) false false)
      (`SceneComponent.K2_SetRelativeLocation` (`self.Scene`) (`KismetMathLibrary.MakeVector` 0.0 0.0 _newtrack_2) false false)
      (`SceneComponent.K2_SetRelativeLocation` (`self.StaticMesh`) (`KismetMathLibrary.MakeVector` 0.0 0.0 _newtrack_3) false false))
    (:`Finished`
      (`SceneComponent.SetVisibility` (`self.StaticMesh`) false false)
      (`NiagaraFunctionLibrary.SpawnSystemAtLocation` "/Game/GameJam/Blueprints/Item/NewNiagaraEmitter_System.NewNiagaraEmitter_System" (`SceneComponent.K2_GetComponentLocation` (`self.StaticMesh`)))
      (`GameplayStatics.PlaySound2D` "/Game/GameJam/Blueprints/Item/Sound_coins.Sound_coins" 1.0 1.0 0.0 null null))))

(fn `Triggered`
  (`self.CustomEvent_0`)
  (`parent.Triggered`))

(fn `UserConstructionScript`
  (`parent.UserConstructionScript`))