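; BP_Button is a one-shot button that opens gates and activates platforms when any Character overlaps its box.
; It sends InterOpenGateMessage to all actors matching its GateTag and PlatformTag, then fires the Triggered dispatcher.
; A timeline moves the top mesh along Z from its starting location while a dynamic material raises its emissive glow.
; The press also plays a stinger sound and disables box collision to prevent retriggering.
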(event `self.ReceiveBeginPlay`
  (set `self.Tem_Relative Location` (`SceneComponent.RelativeLocation` (`self.StaticMesh_Up`)))
  (bind _returnvalue (`PrimitiveComponent.CreateDynamicMaterialInstance` (`self.StaticMesh_Up`) 0 (`PrimitiveComponent.GetMaterial` (`self.StaticMesh_Up`) 0) "None"))
  (set `self.MaterialInstance` _returnvalue)
  (`MaterialInstanceDynamic.SetScalarParameterValue` (`self.MaterialInstance`) "EmissIntensity" 0.04))

(event `self.Box.OnComponentBeginOverlap`
  (params (OverlappedComponent :type "PrimitiveComponent Object Reference") (OtherActor :type "Actor Object Reference") (OtherComp :type "PrimitiveComponent Object Reference") (OtherBodyIndex :type Integer) (bFromSweep :type Boolean) (SweepResult :type "HitResult Structure (by ref)"))
  (bind (_tem_relative_location_x _tem_relative_location_y _tem_relative_location_z) (`KismetMathLibrary.BreakVector` (`self.Tem_Relative Location`)))
  (cast `Character` OtherActor)
  (`|ExecutionSequence`
    (:`then_0`
      (bind _outactors (`GameplayStatics.GetAllActorsWithTag` (`self.Gate_Tag`)))
      (for _array_element _outactors
        (message `/Game/GameJam/Blueprints/Item/Inter_Gate.Inter_OpenGate` _array_element false)))
    (:`then_1`
      (bind _outactors_2 (`GameplayStatics.GetAllActorsWithTag` (`self.Platform_Tag`)))
      (for _array_element_2 _outactors_2
        (message `/Game/GameJam/Blueprints/Item/Inter_Gate.Inter_OpenGate` _array_element_2 false)))
    (:`then_2`
      (bind (_direction _location _material) (`Timeline|Timeline_0` :!via `PlayFromStart`)
        (:`Update`
          (`SceneComponent.K2_SetRelativeLocation` (`self.StaticMesh_Up`) (`KismetMathLibrary.MakeVector` _tem_relative_location_x _tem_relative_location_y (+ _location _tem_relative_location_z)) true false)
          (`MaterialInstanceDynamic.SetScalarParameterValue` (`self.MaterialInstance`) "EmissIntensity" 10.0))))
    (:`then_3`
      (`PrimitiveComponent.SetCollisionEnabled` (`self.Box`) "NoCollision")
      (`GameplayStatics.PlaySound2D` "/Game/GameJam/Wav/FM_Short_Positive_Stinger_1.FM_Short_Positive_Stinger_1" 0.7 1.0 0.0 null null))
    (:`then_4`
      (`self.Triggered`))))

(fn `UserConstructionScript`)