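; BP_SendBackPlatform is a spline-following moving platform that a linked BP_Button enables, also making a second mesh visible.
; Once enabled, a BP_TestCharacter entering the box starts movement after a stay timer, with Tick advancing the mesh at constant speed.
; It travels forward only while the character is aboard, heading back shortly after they leave.
; Timed toggles reverse it at the start and, with CanAutoBack, at the end.
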(event `self.ReceiveBeginPlay`
  (set `self.SplineLength` (`SplineComponent.GetSplineLength` (`self.Spline`)))
  (bind _targetactor (`self.TargetActor`)
    (:`then`
      (bind _asbp_button (cast `/Game/GameJam/Blueprints/Item/BP_Button` _targetactor))
      (add `/Game/GameJam/Blueprints/Item/BP_Button.Triggered` _asbp_button (delegate `OnBindTriggered`)))
    (:`else`)))

(event `OnBindTriggered`
  (set `self.CanMove` true)
  (`SceneComponent.SetVisibility` (`self.StaticMesh1`) true false))

(event `self.ReceiveTick`
  (params (DeltaSeconds :type "Float (single-precision)"))
  (`self.UpdateMovement` DeltaSeconds))

(event `self.Box.OnComponentBeginOverlap`
  (params (OverlappedComponent :type "PrimitiveComponent Object Reference") (OtherActor :type "Actor Object Reference") (OtherComp :type "PrimitiveComponent Object Reference") (OtherBodyIndex :type Integer) (bFromSweep :type Boolean) (SweepResult :type "HitResult Structure (by ref)"))
  (bind _asbp_test_character (cast `/Game/GameJam/Blueprints/Character/BP_TestCharacter` OtherActor))
  (set `self.As BP Test Character` _asbp_test_character)
  (if (`self.CanMove`)
    (`KismetSystemLibrary.K2_SetTimer` null "SetStartUpdate" (`self.StayTime`))))

(event `self.Box.OnComponentEndOverlap`
  (params (OverlappedComponent :type "PrimitiveComponent Object Reference") (OtherActor :type "Actor Object Reference") (OtherComp :type "PrimitiveComponent Object Reference") (OtherBodyIndex :type Integer))
  (cast `/Game/GameJam/Blueprints/Character/BP_TestCharacter` OtherActor)
  (set `self.As BP Test Character` null)
  (`KismetSystemLibrary.Delay` 1.0)
  (`self.SetStartToFinish` false))

(fn `SetStartToFinish`
  (params (MoveStartToFinish :type Boolean))
  (if MoveStartToFinish
    (`self.As BP Test Character`
      (:`then`
        (set `self.MoveStartToFinish` MoveStartToFinish))
      (:`else`
        (set `self.MoveStartToFinish` false)))
    (else
      (set `self.MoveStartToFinish` MoveStartToFinish))))

(fn `SetStartUpdate`
  (set `self.StartUpdate` true)
  (`self.SetStartToFinish` true))

(fn `StartToggleDirection`
  (`self.SetStartToFinish` (not (`self.MoveStartToFinish`))))

(fn `ToggleDirection`
  (if (not (> (`KismetSystemLibrary.K2_GetTimerRemainingTimeHandle` (`self.ToggleTimer`)) 0.0))
    (bind _returnvalue (`KismetSystemLibrary.K2_SetTimer` null "StartToggleDirection" (`self.StayTime`)))
    (set `self.ToggleTimer` _returnvalue)))

(fn `UpdateMovement`
  (params (`Delta Seconds` :type "Float (single-precision)"))
  (bind _returnvalue (+ (`self.CurrentDistance`) (* (`self.SpeedPerSecond`) (`self.Delta Seconds`))))
  (bind _returnvalue_2 (- (`self.CurrentDistance`) (* (`self.SpeedPerSecond`) (`self.Delta Seconds`))))
  (if (`self.StartUpdate`)
    (set `self.Delta Seconds` `Delta Seconds`)
    (if (`self.MoveStartToFinish`)
      (if (<= _returnvalue (`self.SplineLength`))
        (set `self.CurrentDistance` _returnvalue)
        (`SceneComponent.K2_SetWorldLocation` (`self.StaticMesh`) (`SplineComponent.GetLocationAtDistanceAlongSpline` (`self.Spline`) (`self.CurrentDistance`) "World") false false)
        (else
          (set `self.CurrentDistance` (`self.SplineLength`))
          (if (`self.CanAutoBack`)
            (`self.ToggleDirection`))))
      (elif (<= _returnvalue_2 0.0)
        (set `self.CurrentDistance` 0.0)
        (`self.ToggleDirection`)
        (else
          (set `self.CurrentDistance` _returnvalue_2)
          (`SceneComponent.K2_SetWorldLocation` (`self.StaticMesh`) (`SplineComponent.GetLocationAtDistanceAlongSpline` (`self.Spline`) (`self.CurrentDistance`) "World") false false))))))

(fn `UserConstructionScript`)