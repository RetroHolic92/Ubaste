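; Actor component for BP_TestCharacter that spawns Niagara movement effects and sounds for walking, jumping and landing at the character's feet.
; A looping timer spawns walk VFX and sound while the character moves on the ground.
; It binds to the character's jump event for jump effects.
; Tick compares the previous falling state with the current one to detect landing, which reuses the jump system without sound.
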(event `self.ReceiveBeginPlay`
  (bind _asbp_test_character (cast `/Game/GameJam/Blueprints/Character/BP_TestCharacter` (`self.GetOwner`)))
  (bind _output_get (set `self.As BP Test Character` _asbp_test_character))
  (set `self.Movement` (`Pawn.GetMovementComponent` _output_get))
  (`KismetSystemLibrary.K2_SetTimer` null "SpawnWalkVFX" 0.3 true)
  (add `/Game/GameJam/Blueprints/Character/BP_TestCharacter.JumpEvent` _output_get (`|CreateDelegate` :!event `PlayJumpVFX`)))

(event `self.ReceiveTick`
  (params (DeltaSeconds :type "Float (single-precision)"))
  (`|ExecutionSequence`
    (:`then_0`
      (if (`self.IsFalling`)
        (if (== (`NavMovementComponent.IsFalling` (`self.Movement`)) false)
          (`self.PlayLandVFX`))))
    (:`then_1`
      (set `self.IsFalling` (`NavMovementComponent.IsFalling` (`self.Movement`))))))

(fn `PlayJumpVFX`
  (bind _returnvalue (`Actor.K2_GetActorLocation` (`self.As BP Test Character`)))
  (bind _returnvalue_2 (`NavMovementComponent.IsFalling` (`self.Movement`)))
  (`KismetSystemLibrary.PrintString` (`KismetStringLibrary.Conv_BoolToString` _returnvalue_2))
  (if (not _returnvalue_2)
    (`NiagaraFunctionLibrary.SpawnSystemAtLocation` "/Game/GameJam/VFXs/NGS_Jump.NGS_Jump" (- _returnvalue (0.0 0.0 60.0)))
    (`GameplayStatics.PlaySoundAtLocation` "/Game/GameJam/Audio/jump.jump" _returnvalue (struct) 1.0 1.0 0.0 null null null null)))

(fn `PlayLandVFX`
  (bind _returnvalue (`NavMovementComponent.IsFalling` (`self.Movement`)))
  (`KismetSystemLibrary.PrintString` (`KismetStringLibrary.Conv_BoolToString` _returnvalue))
  (if (not _returnvalue)
    (`NiagaraFunctionLibrary.SpawnSystemAtLocation` "/Game/GameJam/VFXs/NGS_Jump.NGS_Jump" (- (`Actor.K2_GetActorLocation` (`self.As BP Test Character`)) (0.0 0.0 60.0)))))

(fn `SpawnWalkVFX`
  (bind _returnvalue (`Actor.K2_GetActorLocation` (`self.As BP Test Character`)))
  (bind _movement (`self.Movement`)
    (:`then`
      (if (`NavMovementComponent.IsFalling` _movement)
        _
        (elif (!= (`MovementComponent.Velocity` _movement) (0.0 0.0 0.0))
          (`NiagaraFunctionLibrary.SpawnSystemAtLocation` "/Game/GameJam/VFXs/NGS_Walk.NGS_Walk" (- _returnvalue (0.0 0.0 60.0)))
          (`GameplayStatics.PlaySoundAtLocation` "/Game/GameJam/Audio/Walk.Walk" _returnvalue (struct) 1.0 1.0 0.0 null null null null))))
    (:`else`)))