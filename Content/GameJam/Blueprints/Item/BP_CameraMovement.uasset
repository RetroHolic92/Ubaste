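; BP_CameraMovement is a trigger box that briefly shows a tagged actor through the player camera, then returns to the character.
; On overlap by BP_TestCharacter or BP_GhostCharacter, it freezes that character's input and runs delayed view-target blends on player controller 0.
; The target is the first actor found with the configured tag.
; IsMoved makes it one-shot but is only set after the return blend starts.
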(event `self.Box.OnComponentBeginOverlap`
  (params (OverlappedComponent :type "PrimitiveComponent Object Reference") (OtherActor :type "Actor Object Reference") (OtherComp :type "PrimitiveComponent Object Reference") (OtherBodyIndex :type Integer) (bFromSweep :type Boolean) (SweepResult :type "HitResult Structure (by ref)"))
  (if (not (`self.IsMoved`))
    (bind _asbp_test_character (cast `/Game/GameJam/Blueprints/Character/BP_TestCharacter` OtherActor)
      (:`then`
        (bind _outactors (`GameplayStatics.GetAllActorsWithTag` (`self.Tag`)))
        (if (!= (`KismetArrayLibrary.Array_Length` _outactors) 0)
          (`/Game/GameJam/Blueprints/Character/BP_TestCharacter.FreezeInput` _asbp_test_character (`self.Freeze Time`))
          (`KismetSystemLibrary.Delay` (`self.DelayShowTime`))
          (`PlayerController.SetViewTargetWithBlend` (`GameplayStatics.GetPlayerController` 0) (`|GetArrayItem` _outactors) (`self.Blend Time Intro`) "VTBlend_Linear" 0.0 false)
          (`KismetSystemLibrary.Delay` (`self.ShowTime`))
          (`PlayerController.SetViewTargetWithBlend` (`GameplayStatics.GetPlayerController` 0) _asbp_test_character (`self.Blend Time Outro`) "VTBlend_Linear" 0.0 false)
          (set `self.IsMoved` true :!label _label)))
      (:`CastFailed`
        (bind _asbp_ghost_character (cast `/Game/GameJam/Blueprints/Character/BP_GhostCharacter` OtherActor))
        (bind _outactors_2 (`GameplayStatics.GetAllActorsWithTag` (`self.Tag`)))
        (if (!= (`KismetArrayLibrary.Array_Length` _outactors_2) 0)
          (`/Game/GameJam/Blueprints/Character/BP_GhostCharacter.FreezeInput` _asbp_ghost_character (`self.Freeze Time`))
          (`KismetSystemLibrary.Delay` (`self.DelayShowTime`))
          (`PlayerController.SetViewTargetWithBlend` (`GameplayStatics.GetPlayerController` 0) (`|GetArrayItem` _outactors_2) (`self.Blend Time Outro`) "VTBlend_Linear" 0.0 false)
          (`KismetSystemLibrary.Delay` (`self.ShowTime`))
          (`PlayerController.SetViewTargetWithBlend` (`GameplayStatics.GetPlayerController` 0) _asbp_ghost_character 0.8 "VTBlend_Linear" 0.0 false)
          (goto _label))))))

(fn `UserConstructionScript`)