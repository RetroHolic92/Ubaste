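; BP_HitZone_All is a placeable kill zone that affects both the test character and the ghost character.
; When either character begins overlapping its Box, the zone calls SetDeath on it, trying the test character cast first.
; SwitchMode shows the Cube and TextRender markers only in build mode, hiding them otherwise.
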(event `self.Box.OnComponentBeginOverlap`
  (params (OverlappedComponent :type "PrimitiveComponent Object Reference") (OtherActor :type "Actor Object Reference") (OtherComp :type "PrimitiveComponent Object Reference") (OtherBodyIndex :type Integer) (bFromSweep :type Boolean) (SweepResult :type "HitResult Structure (by ref)"))
  (bind _asbp_test_character (cast `/Game/GameJam/Blueprints/Character/BP_TestCharacter` OtherActor)
    (:`then`
      (`/Game/GameJam/Blueprints/Character/BP_TestCharacter.SetDeath` _asbp_test_character true))
    (:`CastFailed`
      (bind _asbp_ghost_character (cast `/Game/GameJam/Blueprints/Character/BP_GhostCharacter` OtherActor))
      (`/Game/GameJam/Blueprints/Character/BP_GhostCharacter.SetDeath` _asbp_ghost_character true))))

(event `/Game/GameJam/Blueprints/Interface/I_SwitchBuildMode.SwitchMode`
  (params (IsBuildMode :type Boolean))
  (`SceneComponent.SetVisibility` (`self.Cube`) IsBuildMode false)
  (`SceneComponent.SetVisibility` (`self.TextRender`) IsBuildMode false))

(fn `ComponentsToSave`
  (returns (Components :type "Array of ActorComponent Object Reference"))
  (return))

(fn `UserConstructionScript`)