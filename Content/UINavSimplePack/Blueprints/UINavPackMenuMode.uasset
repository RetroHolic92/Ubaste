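; Menu mode Blueprint for the UINav pack that starts a background music track at half volume on BeginPlay.
; It also holds an unconnected, never-executed save bootstrap that polls until a Steam ID is available and uses it as the slot name.
; If no save exists, that dormant logic creates a BP_SaveGameBase, seeds pass and speed entries for each DT_LevelList row, then saves it.
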(event `self.ReceiveBeginPlay`
  (`|ExecutionSequence`
    (:`then_0`
      (`GameplayStatics.PlaySound2D` "/Game/FarmMusicPack/Music/wav/FM_Playlist_Music_1-3_FULL_Loop.FM_Playlist_Music_1-3_FULL_Loop" 0.5 1.0 0.0 null null))))

(fn `UserConstructionScript`)