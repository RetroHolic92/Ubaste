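; BP_ClownPlatform is a moving bounce platform item that launches the ghost character upward on contact.
; The construction script builds two relative InterpToMovement control points from start and end locations and sets the travel duration.
; When BP_GhostCharacter enters its box trigger, it launches the character with a configurable Z velocity, overriding existing velocity, and plays a 2D jump sound.
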(event `self.Box.OnComponentBeginOverlap`
  (params (OverlappedComponent :type "PrimitiveComponent Object Reference") (OtherActor :type "Actor Object Reference") (OtherComp :type "PrimitiveComponent Object Reference") (OtherBodyIndex :type Integer) (bFromSweep :type Boolean) (SweepResult :type "HitResult Structure (by ref)"))
  (bind _asbp_ghost_character (cast `/Game/GameJam/Blueprints/Character/BP_GhostCharacter` OtherActor))
  (`Character.LaunchCharacter` _asbp_ghost_character (`KismetMathLibrary.MakeVector` 0.0 0.0 (`self.Launch Velocity Z`)) true true)
  (`GameplayStatics.PlaySound2D` "/Game/GameJam/Audio/jump.jump" 1.0 1.0 0.0 null null))

(fn `UserConstructionScript`
  (bind _interptomovement (`self.InterpToMovement`))
  (set `InterpToMovementComponent.ControlPoints` (`|MakeArray` (make `InterpControlPoint` (`self.LocationStart`)) (make `InterpControlPoint` (`self.LocationEnd`))) _interptomovement)
  (set `InterpToMovementComponent.Duration` (`self.Duration`) _interptomovement))