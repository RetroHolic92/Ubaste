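; BP_Gate is a gate actor that swings its static mesh open by animating relative yaw rotation.
; InterOpenGate waits for a configurable DelayTime, then plays a timeline from the start to drive the yaw.
; CE_StartRotation follows the same delay-then-timeline pattern with its own separate timeline, giving a second rotation motion.
; Both are triggered externally, as BeginPlay and the construction script are empty.
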(event `self.ReceiveBeginPlay`)

(event `/Game/GameJam/Blueprints/Item/Inter_Gate.Inter_OpenGate`
  (params (ID :type Boolean))
  (`KismetSystemLibrary.Delay` (`self.DelayTime`))
  (bind (_direction _newtrack_0) (`Timeline|Timeline_0` :!via `PlayFromStart`)
    (:`Update`
      (`SceneComponent.K2_SetRelativeRotation` (`self.StaticMesh`) (`KismetMathLibrary.MakeRotator` 0.0 0.0 _newtrack_0) false false))))

(event `CE_StartRotation`
  (`KismetSystemLibrary.Delay` (`self.DelayTime`))
  (bind (_direction _newtrack_0) (`Timeline|Timeline_1` :!via `PlayFromStart`)
    (:`Update`
      (`SceneComponent.K2_SetRelativeRotation` (`self.StaticMesh`) (`KismetMathLibrary.MakeRotator` 0.0 0.0 _newtrack_0) false false))))

(fn `UserConstructionScript`)